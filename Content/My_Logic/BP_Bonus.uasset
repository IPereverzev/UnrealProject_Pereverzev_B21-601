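; BP_Bonus is a moving bonus pickup that spawns two BP_Spher actors when its Cube hits a BP_Platform.
; Tick offsets the actor along X by V each frame, with no delta-time scaling.
; The Cube's hit event prints a debug "Hello", then a Sequence runs the same spawn twice at the Cube's transform, adjusting for collisions, before destroying the bonus.
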(event `self.ReceiveTick`
  (params (DeltaSeconds :type "Float (single-precision)"))
  (`self.K2_AddActorWorldOffset` (`KismetMathLibrary.MakeVector` (`self.V`) 0.0 0.0)))

(event `self.Cube.OnComponentHit`
  (params (HitComponent :type "PrimitiveComponent Object Reference") (OtherActor :type "Actor Object Reference") (OtherComp :type "PrimitiveComponent Object Reference") (NormalImpulse :type "Vector Structure") (Hit :type "HitResult Structure (by ref)"))
  (if (== OtherActor "/Game/My_Logic/BP_Platform.BP_Platform")
    (`KismetSystemLibrary.PrintString` "Hello")
    (`|ExecutionSequence`
      (:`then_0`
        (`|SpawnActorFromClass` "/Game/My_Logic/BP_Spher.BP_Spher_C" (`SceneComponent.K2_GetComponentToWorld` (`self.Cube`)) "AdjustIfPossibleButAlwaysSpawn" "OverrideRootScale" null null :!label _label))
      (:`then_1`
        (goto _label))
      (:`then_2`
        (`self.K2_DestroyActor`)))))

(fn `UserConstructionScript`)