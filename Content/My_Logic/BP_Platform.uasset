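; BP_Platform is a player-controlled platform that slides along the world Y axis from MoveRight input.
; Two handlers of the same axis read only the input's sign, moving it toward +Y for negative and -Y for positive values.
; Each step is a fixed DeltaLocationY offset, not scaled by frame time.
; Event_SlowMod temporarily lowers that step, then sets a hard-coded faster value after a delay.
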(event `InputAxis|MoveRight`
  (params (AxisValue :type "Float (single-precision)"))
  (if (< AxisValue 0.0)
    (`self.K2_AddActorWorldOffset` (`KismetMathLibrary.MakeVector` 0.0 (`self.Delta Location Y`)))))

(event `InputAxis|MoveRight`
  (params (AxisValue :type "Float (single-precision)"))
  (if (> AxisValue 0.0)
    (`self.K2_AddActorWorldOffset` (`KismetMathLibrary.MakeVector` 0.0 (* -1 (`self.Delta Location Y`))))))

(event `Event_SlowMod`
  (set `self.Delta Location Y` 10.0)
  (`KismetSystemLibrary.Delay` 10.0)
  (set `self.Delta Location Y` 50.0))

(fn `UserConstructionScript`)